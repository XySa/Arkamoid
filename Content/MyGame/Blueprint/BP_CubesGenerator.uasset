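; BP_CubesGenerator is an actor that spawns a randomly sized grid of BP_Cube_Child cubes and tracks their destruction.
; On BeginPlay it spawns the padded grid from its location, binds each cube's death event and sets the win count to the total.
; Each death adds score to BP_MyPlayerState, cached after a delay, and reaching the count fires AllCubesDied.
; Construction-script preview meshes and their cleanup are disconnected.
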(event `self.ReceiveBeginPlay`
  (bind (_returnvalue_x _returnvalue_y _returnvalue_z) (`KismetMathLibrary.BreakVector` (`self.K2_GetActorLocation`)))
  (`|ExecutionSequence`
    (:`then_0`
      (`KismetSystemLibrary.Delay` 3.0)
      (bind _asbp_my_player_state (cast `/Game/MyGame/Blueprint/Core/BP_MyPlayerState` (`GameplayStatics.GetPlayerState` 0)))
      (set `self.As BP My Player State` _asbp_my_player_state))
    (:`then_1`
      (for _index (range 1 (+ (`KismetMathLibrary.RandomIntegerInRange` 1 3) 1))
        (for _index_2 (range 1 (+ (`KismetMathLibrary.RandomIntegerInRange` 1 11) 1))
          (bind _returnvalue (`|SpawnActorFromClass` "/Game/MyGame/Blueprint/BP_Cube_Child.BP_Cube_Child_C" (`KismetMathLibrary.MakeTransform` (`KismetMathLibrary.MakeVector` (+ _returnvalue_x (`KismetMathLibrary.Conv_IntToDouble` (* _index (`self.Padding`)))) (+ (`KismetMathLibrary.Conv_IntToDouble` (* _index_2 (`self.Padding`))) _returnvalue_y) _returnvalue_z)) "Undefined" "OverrideRootScale" null null))
          (`KismetArrayLibrary.Array_Add` (`self.CubesArray`) _returnvalue)))
      (bind _amountcubes (`self.GetCubesForWin`))
      (set `self.AmountCubesForWin` _amountcubes)
      (for _array_element (`self.CubesArray`)
        (add `/Game/MyGame/Blueprint/BP_Cube_Parent.CubeDead` _array_element (delegate `CubeDead`))))))

(event `CubeDead`
  (params (Score :type Integer))
  (bind _as_bp_my_player_state (`self.As BP My Player State`))
  (bind _deadcubes (`self.DeadCubes`))
  (if (`KismetSystemLibrary.IsValid` _as_bp_my_player_state)
    (`/Game/MyGame/Blueprint/Core/BP_MyPlayerState.AddedScore` _as_bp_my_player_state Score)
    (`/Engine/EditorBlueprintResources/StandardMacros.IncrementInt` _deadcubes
      (:`  `
        (if (>= _deadcubes (`self.AmountCubesForWin`))
          (`self.AllCubesDied`))))))

(fn `GetCubesForWin`
  (returns (AmountCubes :type Integer))
  (return (`KismetArrayLibrary.Array_Length` (`self.CubesArray`))))

(fn `UserConstructionScript`)