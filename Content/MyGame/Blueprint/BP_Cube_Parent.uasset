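; BP_Cube_Parent is a breakable cube, named as a parent class, that takes one or two ball hits to destroy.
; The Construction Script randomly picks its Lives and sets a silver material for one life or gold for two.
; A Hit from a BP_Ball calls BallIsHit, which decrements Lives and destroys the actor when none remain.
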(event `self.ReceiveBeginPlay`)

(event `self.ReceiveHit`
  (params (MyComp :type "PrimitiveComponent Object Reference") (Other :type "Actor Object Reference") (OtherComp :type "PrimitiveComponent Object Reference") (bSelfMoved :type Boolean) (HitLocation :type "Vector Structure") (HitNormal :type "Vector Structure") (NormalImpulse :type "Vector Structure") (Hit :type "HitResult Structure (by ref)"))
  (cast `/Game/MyGame/Blueprint/BP_Ball` Other)
  (`self.BallIsHit`))

(event `BallIsHit`
  (bind _result (`/Engine/EditorBlueprintResources/StandardMacros.DecrementInt` (`self.Lives`))
    (:`  `
      (if (<= _result 0)
        (`self.K2_DestroyActor`)))))

(fn `UserConstructionScript`
  (bind _cube (`self.Cube`))
  (bind _output_get (set `self.Lives` (`KismetMathLibrary.RandomIntegerInRange` 1 2)))
  (switch `int` _output_get
    (:`1`
      (`PrimitiveComponent.SetMaterial` _cube 0 "/Game/MyGame/Material/Metals/M_Metal_Silver.M_Metal_Silver"))
    (:`2`
      (`PrimitiveComponent.SetMaterial` _cube 0 "/Game/MyGame/Material/Metals/M_Metal_Gold.M_Metal_Gold"))))