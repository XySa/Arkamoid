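; BP_Ball is a ball actor that moves itself along a direction vector and bounces off whatever it hits.
; Each Tick applies a swept world offset from Direction, Speed and delta time, without physics simulation.
; On a blocking hit it reflects Direction about the hit normal and raises Speed by AddedSpeed up to a fixed cap, so play speeds up with each bounce.
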(event `self.ReceiveTick`
  (params (DeltaSeconds :type "Float (single-precision)"))
  (bind _speed (`self.Speed`))
  (bind (_returnvalue_x _returnvalue_y _returnvalue_z) (`KismetMathLibrary.BreakVector` (* (* DeltaSeconds (`self.Speed`)) (`self.Direction`))))
  ;[0 0 0] Speed ball
  (bind _sweephitresult (`self.K2_AddActorWorldOffset` (`KismetMathLibrary.MakeVector` _returnvalue_x _returnvalue_y _returnvalue_z) true))
  (bind (_bblockinghit _binitialoverlap _time _distance _location _impactpoint _normal) (`GameplayStatics.BreakHitResult` _sweephitresult))
  (if _bblockinghit
    (set `self.Direction` (`KismetMathLibrary.GetReflectionVector` (`self.Direction`) _normal))
    (if (< _speed 4000.0)
      (set `self.Speed` (`KismetMathLibrary.FMin` (+ _speed (`self.AddedSpeed`)) 4000.0)))))

(fn `UserConstructionScript`)