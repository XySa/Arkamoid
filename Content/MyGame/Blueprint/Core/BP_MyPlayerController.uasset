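; Player controller for a ball-and-cubes game that owns the HUD, forwards input and handles win or lose.
; Left/right and spawn-ball input go through server-named events to sweep-move the pawn along Y and spawn balls; the follow-up multicast move passes a zero axis.
; The pawn's game-end event and the cube generator's all-cubes-died event share one end path that collapses the HUD and shows the result screen with UI-only input.
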(event `self.ReceiveBeginPlay`
  (`|ExecutionSequence`
    (:`then_0`
      (if (`self.IsLocalPlayerController`)
        (`WidgetBlueprintLibrary.SetInputMode_GameOnly` self)
        (bind _returnvalue (`|CreateWidget` "/Game/MyGame/Ui/WBP_HUD.WBP_HUD_C" self))
        (`UserWidget.AddToViewport` _returnvalue 0)
        (set `self.HUD` _returnvalue)))
    (:`then_1`
      (bind _returnvalue_2 (`GameplayStatics.GetActorOfClass` "/Game/MyGame/Blueprint/BP_CubesGenerator.BP_CubesGenerator_C"))
      (add `/Game/MyGame/Blueprint/BP_CubesGenerator.AllCubesDied` _returnvalue_2 (delegate `GameFinished`)))))

(event `self.ReceivePossess`
  (params (PossessedPawn :type "Pawn Object Reference"))
  (bind _asbp_my_pawn (cast `/Game/MyGame/Blueprint/Core/BP_MyPawn` PossessedPawn))
  (add `/Game/MyGame/Blueprint/Core/BP_MyPawn.GameEnd` _asbp_my_pawn (delegate `PlayerDie`)))

(event `PlayerDie`
  (set `self.bIsWinner` false)
  (`Widget.SetVisibility` (`self.HUD`) "Collapsed" :!label _label)
  (bind _returnvalue (`|CreateWidget` "/Game/MyGame/Ui/WBP_WINScreen.WBP_WINScreen_C" self))
  (`/Game/MyGame/Ui/WBP_WINScreen.UpdateWinner` _returnvalue (`self.bIsWinner`))
  (`UserWidget.AddToViewport` _returnvalue 0)
  (`WidgetBlueprintLibrary.SetInputMode_UIOnlyEx` self _returnvalue)
  (set `self.bShowMouseCursor` true))

(event `GameFinished`
  (set `self.bIsWinner` true)
  (if (`self.IsLocalPlayerController`)
    (goto _label)))

(event `InputAxis|Left_Right`
  (params (AxisValue :type "Float (single-precision)"))
  (`self.Server_Move_LeftRight` AxisValue))

(event `InputAction|SpawnBall`
  (params (Key :type "Key Structure"))
  (:`Pressed`
    (`self.Server SpawnBall Event`)))

(event `Server_Move_LeftRight`
  (params (`Axis Value` :type "Float (double-precision)"))
  (`self.K2_AddActorWorldOffset` (`self.K2_GetPawn`) (`KismetMathLibrary.MakeVector` 0.0 (* (`GameplayStatics.GetWorldDeltaSeconds`) `Axis Value` (`self.Speed`))) true false)
  (`self.Multicast Move Event` 0.0))

(event `Server SpawnBall Event`
  (bind _asbp_my_pawn (cast `/Game/MyGame/Blueprint/Core/BP_MyPawn` (`self.K2_GetPawn`)))
  (`/Game/MyGame/Blueprint/Core/BP_MyPawn.SpawnBall` _asbp_my_pawn))

(event `Multicast Move Event`
  (params (`Axis Value` :type "Float (double-precision)"))
  (`self.K2_AddActorWorldOffset` (`self.K2_GetPawn`) (`KismetMathLibrary.MakeVector` 0.0 (* (`GameplayStatics.GetWorldDeltaSeconds`) `Axis Value` (`self.Speed`))) true false))

(fn `UserConstructionScript`)