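; BP_MyPlayerState is a player state that holds the player's total score, lives and game-end flag.
; On BeginPlay it binds to score, lives and game-end events on player 0's BP_MyPawn, then stores and rebroadcasts each change.
; Incoming score values are added to the running total rather than replacing it.
; AddedScore also raises the total by an absolute amount and broadcasts the change.
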(event `self.ReceiveBeginPlay`
  (bind _asbp_my_pawn (cast `/Game/MyGame/Blueprint/Core/BP_MyPawn` (`GameplayStatics.GetPlayerPawn` 0)))
  (add `/Game/MyGame/Blueprint/Core/BP_MyPawn.ScoreChanged` _asbp_my_pawn (delegate `PlayersscoreChanged`))
  (add `/Game/MyGame/Blueprint/Core/BP_MyPawn.LivesChanged` _asbp_my_pawn (delegate `Player LivesChanged`))
  (add `/Game/MyGame/Blueprint/Core/BP_MyPawn.GameEnd` _asbp_my_pawn (delegate `GameEndEvent`)))

(event `PlayersscoreChanged`
  (params (CurrentScore :type Integer))
  (bind _output_get (set `self.All Score` (+ CurrentScore (`self.All Score`))))
  (`self.ScoreChanged` _output_get))

(event `Player LivesChanged`
  (params (AmountLives :type Integer))
  (bind _output_get (set `self.Player Lives` AmountLives))
  (`self.LivesChanged` _output_get))

(event `GameEndEvent`
  (params (bGameEnd :type Boolean))
  (bind _output_get (set `self.bGameEnd` bGameEnd))
  (`self.GameEnd` _output_get))

(fn `AddedScore`
  (params (Amount :type Integer))
  (bind _output_get (set `self.All Score` (+ (`self.All Score`) (`KismetMathLibrary.Abs_Int` Amount))))
  (`self.ScoreChanged` _output_get))

(fn `UserConstructionScript`)